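; BP_NPC is a non-player character that shows dialogue when the player enters its sphere trigger.
; It creates a WBP_Dialogue widget at BeginPlay, shows it on overlap and removes it on exit.
; It registers itself on BP_ThirdPersonCharacter, while NextLineText writes the current Dialogue entry to the textbox.
; The line index has a hard-coded limit, after which the widget closes, and never resets.
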(event OnComponentBeginOverlap(Sphere)
  (params (OverlappedComponent :type Primitive%20Component%20Object%20Reference) (OtherActor :type Actor%20Object%20Reference) (OtherComp :type Primitive%20Component%20Object%20Reference) (OtherBodyIndex :type Integer) (bFromSweep :type Boolean) (SweepResult :type Hit%20Result%20Structure%20%28by%20ref%29))
  (bind _asbp_third_person_character (Utilities|Casting|CastToBP_ThirdPersonCharacter OtherActor))
  (bind _output_get (Variables|Default|SetPlayer%20Ref _asbp_third_person_character))
  (Variables|/Game/ThirdPerson/Blueprints/BP_ThirdPersonCharacter.BP_ThirdPersonCharacter_C|SetNPC _output_get self)
  (UserInterface|Viewport|AddtoViewport (Variables|Default|GetDialogue%20Ref) 0)
  (CallFunction|NextLineText))

(event OnComponentEndOverlap(Sphere)
  (params (OverlappedComponent :type Primitive%20Component%20Object%20Reference) (OtherActor :type Actor%20Object%20Reference) (OtherComp :type Primitive%20Component%20Object%20Reference) (OtherBodyIndex :type Integer))
  (Utilities|Casting|CastToBP_ThirdPersonCharacter OtherActor)
  (Widget|RemovefromParent (Variables|Default|GetDialogue%20Ref)))

(event Custom|Next%20Line%20Text
  (bind _lineindex (Variables|Default|GetLineIndex))
  (Rendering|Components|TextRender|SetText (Variables|/Game/Blueprints/WBP_Dialogue.WBP_Dialogue_C|GetNPCTextbox (Variables|Default|GetDialogue%20Ref)) (Utilities|Array|Get(acopy) (Variables|Default|GetDialogue) (Variables|Default|GetLineIndex)))
  (if (<= _lineindex 3)
    (Math|Integer|IncrementInt _lineindex)
    (else
      (Widget|RemovefromParent (Variables|Default|GetDialogue%20Ref)))))

(event EventBeginPlay
  (bind _returnvalue (UserInterface|CreateWidget "/Game/Blueprints/WBP_Dialogue.WBP_Dialogue_C"))
  (Variables|Default|SetDialogue%20Ref _returnvalue))

(fn ConstructionScript)